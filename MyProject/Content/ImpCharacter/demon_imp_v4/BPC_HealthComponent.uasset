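; Health component Blueprint for the imp character that tracks integer health, damage and healing.
; OnHurt and OnHeal change health by a fixed factor, clamped between minimum and maximum, and print the result to screen while the owner survives or heals.
; Reaching minimum health sends OnDeathMessage to the owner.
; A non-lethal hit triggers a timed invulnerability window, via a flag and Delay, during which further damage is ignored.
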(event Custom|StartInvulnerability
  (Variables|Default|SetisInvurnable true)
  (Utilities|FlowControl|Delay (Variables|Default|GetinvurnabilityDuration))
  (Variables|Default|SetisInvurnable false))

(fn OnHurt
  (if (Variables|Default|GetisInvurnable)
    (return)
    (else
      (bind _output_get (Variables|Default|Sethealth (Math|Integer|Clamp(Integer) (- (Variables|Default|Gethealth) (Variables|Default|GetdamageAndHealingFactor)) (Variables|Default|GetminHealth) (Variables|Default|GetmaxHealth))))
      (if (== (Variables|Default|Gethealth) (Variables|Default|GetminHealth))
        (Class|BPIDeath|OnDeath(Message) (Components|GetOwner))
        (else
          (Development|PrintString (Utilities|String|ToString(Integer) _output_get))
          ;[0.15 0.15 0.15 0.5] Check da samo radi na playeru?
          (CallFunction|StartInvulnerability))))))

(fn OnHeal
  (bind _output_get (Variables|Default|Sethealth (Math|Integer|Clamp(Integer) (+ (Variables|Default|Gethealth) (Variables|Default|GetdamageAndHealingFactor)) (Variables|Default|GetminHealth) (Variables|Default|GetmaxHealth))))
  (Development|PrintString (Utilities|String|ToString(Integer) _output_get)))