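; Ability component for the imp player character, providing a double jump unlock and a throw-aim toggle, with throw firing left as an empty stub.
; BeginPlay caches the owning BP_ImpCharacter's camera boom and its default socket offset.
; Toggling aim switches the target offset, which Tick interpolates toward while printing a debug timestamp.
; Tick starts disabled, turns on when aiming begins and shuts off whenever the offset is within a margin of the default.
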(event EventBeginPlay
  (bind _asbp_imp_character (Utilities|Casting|CastToBP_ImpCharacter (Components|GetOwner)))
  (bind _output_get (Variables|Default|SetPlayerCharacter _asbp_imp_character))
  (bind _output_get_2 (Variables|Default|SetPlayerCameraBoom (Variables|/Game/ImpCharacter/demon_imp_v4/BP_ImpCharacter.BP_ImpCharacter_C|GetCameraBoom _output_get)))
  (bind _output_get_3 (Variables|Default|SetDefaultCameraOffset (Variables|/Script/Engine.SpringArmComponent|GetSocketOffset _output_get_2)))
  (Variables|Default|SetCurrentCameraOffset _output_get_3)
  (Components|Tick|SetComponentTickEnabled false))

(event EventTick
  (params (DeltaSeconds :type Float%20%28single-precision%29))
  (bind _output_get (Variables|Default|SetCurrentCameraOffset (Math|Interpolation|VInterpTo (Variables|Default|GetCurrentCameraOffset) (Variables|Default|GetTargetCameraOffset) DeltaSeconds (Variables|Default|GetCameraBlendSpeed))))
  (Variables|/Script/Engine.SpringArmComponent|SetSocketOffset (Variables|Default|GetPlayerCameraBoom) _output_get)
  (Development|PrintString (Utilities|String|Append "Updating: " (Utilities|String|ToString(Integer) (Math|DateTime|GetMillisecond (Math|DateTime|Now)))))
  (if (<= (Math|Vector|Distance(Vector) (Variables|Default|GetCurrentCameraOffset) (Variables|Default|GetDefaultCameraOffset)) (Variables|Default|GetCameraSocketMarginOfError))
    (Components|Tick|SetComponentTickEnabled false)))

(fn EnableDoubleJump
  (Variables|/Script/Engine.Character|SetJumpMaxCount (Variables|Default|GetPlayerCharacter) 2))

(fn ThrowAim
  (if (Variables|Default|GetisAiming)
    (Variables|Default|SetisAiming false)
    (Variables|Default|SetTargetCameraOffset (Variables|Default|GetDefaultCameraOffset))
    (else
      (Variables|Default|SetisAiming true)
      (Variables|Default|SetTargetCameraOffset (Variables|Default|GetAimCameraOffset))
      (Components|Tick|SetComponentTickEnabled true))))

(fn ThrowFire)