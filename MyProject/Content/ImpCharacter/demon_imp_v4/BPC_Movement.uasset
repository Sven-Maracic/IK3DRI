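; BPC_Movement is a component Blueprint that handles player movement and jumping for the imp character.
; Enhanced Input actions for X and Y movement feed AddMovementInput on player character 0, scaled by MoveDistance.
; Directions come from the right and forward vectors of the player controller's actor rotation.
; The jump action calls Jump on that same character when it starts, fetched globally rather than through the component's owner.
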(event Input|EnhancedActionEvents|EnhancedInputActionIA_XMovement
  (params (ActionValue :type Float%20%28double-precision%29) (ElapsedSeconds :type Float%20%28double-precision%29) (TriggeredSeconds :type Float%20%28double-precision%29) (InputAction :type Input%20Action%20Object%20Reference :default "/Game/ImpCharacter/demon_imp_v4/Inputs/Actions/IA_XMovement.IA_XMovement"))
  (Pawn|Input|AddMovementInput (Game|GetPlayerCharacter 0) (Math|Vector|GetRightVector (Transformation|GetActorRotation (Game|GetPlayerController 0))) (* ActionValue (Variables|Default|GetMoveDistance)) false))

(event Input|EnhancedActionEvents|EnhancedInputActionIA_YMovement
  (params (ActionValue :type Float%20%28double-precision%29) (ElapsedSeconds :type Float%20%28double-precision%29) (TriggeredSeconds :type Float%20%28double-precision%29) (InputAction :type Input%20Action%20Object%20Reference :default "/Game/ImpCharacter/demon_imp_v4/Inputs/Actions/IA_YMovement.IA_YMovement"))
  (Pawn|Input|AddMovementInput (Game|GetPlayerCharacter 0) (Math|Vector|GetForwardVector (Transformation|GetActorRotation (Game|GetPlayerController 0))) (* ActionValue (Variables|Default|GetMoveDistance)) false))

(event Input|EnhancedActionEvents|EnhancedInputActionIA_Jump
  (params (ActionValue :type Boolean) (ElapsedSeconds :type Float%20%28double-precision%29) (TriggeredSeconds :type Float%20%28double-precision%29) (InputAction :type Input%20Action%20Object%20Reference :default "/Game/ImpCharacter/demon_imp_v4/Inputs/Actions/IA_Jump.IA_Jump"))
  (:Started
    (Character|Jump (Game|GetPlayerCharacter 0))))