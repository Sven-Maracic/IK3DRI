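; Actor component for the imp character that adjusts walk speed based on the surface underfoot.
; Every tick it reads the physical material from the CharacterMovement current floor hit, avoiding a separate trace.
; That material maps to a normal, slippery or sticky floor type, which sets MaxWalkSpeed directly: faster on slippery floors, much slower on sticky ones.
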(event EventTick
  (params (DeltaSeconds :type Float%20%28single-precision%29))
  (CallFunction|CheckFloor))

(fn CheckFloor
  (bind _asbp_imp_character (Utilities|Casting|CastToBP_ImpCharacter (Components|GetOwner)))
  (bind _returnedphymaterial (CallFunction|GetFloorTypefromPhysMat (.PhysMat (Collision|BreakHitResult (.HitResult (Utilities|Struct|BreakFindFloorResult (Variables|/Script/Engine.CharacterMovementComponent|GetCurrentFloor (Variables|/Script/Engine.Character|GetCharacterMovement _asbp_imp_character))))))))
  (switch Utilities|FlowControl|Switch|SwitchonE_PhysicalFloorType _returnedphymaterial
    (:NewEnumerator0
      ;[0.15 0.15 0.15 0.5] Should This be somewhere else?
      (Variables|/Script/Engine.CharacterMovementComponent|SetMaxWalkSpeed (Variables|/Script/Engine.Character|GetCharacterMovement _asbp_imp_character) 6e+02))
    (:NewEnumerator1
      (Variables|/Script/Engine.CharacterMovementComponent|SetMaxWalkSpeed (Variables|/Script/Engine.Character|GetCharacterMovement _asbp_imp_character) 1.2e+03))
    (:NewEnumerator2
      (Variables|/Script/Engine.CharacterMovementComponent|SetMaxWalkSpeed (Variables|/Script/Engine.Character|GetCharacterMovement _asbp_imp_character) 1e+02))))

(fn GetFloorTypefromPhysMat
  (params (PhysicalMaterial :type Physical%20Material%20Object%20Reference))
  (if (== PhysicalMaterial "/Game/Materials/PM_SlipperyFloor.PM_SlipperyFloor")
    (return "NewEnumerator1")
    (elif (== PhysicalMaterial "/Game/Materials/PM_StickyFloor.PM_StickyFloor")
      (return "NewEnumerator2")
      (else
        (return "NewEnumerator0")))))