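; BP_PuzzleObject is a puzzle actor that shows an active or inactive state through its material.
; TogglePuzzleState flips IsActive, then ApplyStateVisual has the MaterialSwap component apply the matching material to all slots.
; The construction script puts DefaultMaterial on the first slot of PuzzleMesh.
; BeginPlay sets both MaterialSwap's TargetMesh and PuzzleMesh to None before applying the initial visual.
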(event EventBeginPlay
  (Variables|/Game/BP_MaterialSwapComponent.BP_MaterialSwapComponent_C|SetTargetMesh (Variables|Default|GetMaterialSwap) 0)
  (Variables|Default|SetPuzzleMesh 0)
  (CallFunction|ApplyStateVisual))

(event Collision|EventActorBeginOverlap
  (params (OtherActor :type Actor%20Object%20Reference)))

(event EventTick
  (params (DeltaSeconds :type Float%20%28single-precision%29)))

(fn ConstructionScript
  (Rendering|Material|SetMaterial (Variables|Default|GetPuzzleMesh) 0 "/Engine/EngineMaterials/DefaultMaterial.DefaultMaterial"))

(fn ApplyStateVisual
  (if (Components|Activation|IsActive)
    (Default|ApplyMaterialtoAllSlots (Variables|Default|GetMaterialSwap) (Variables|Default|GetActiveMaterial))
    (else
      (Default|ApplyMaterialtoAllSlots (Variables|Default|GetMaterialSwap) (Variables|Default|GetInactiveMaterial)))))

(fn TogglePuzzleState
  (Variables|Default|SetbIsActive (not (Variables|Default|GetbIsActive)))
  (CallFunction|ApplyStateVisual))