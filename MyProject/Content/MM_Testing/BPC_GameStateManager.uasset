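; Game state manager component that stores the active checkpoint and respawns the player character.
; SetActiveCheckpoint saves a transform and flags that a checkpoint exists.
; RespawnPlayer destroys the current pawn, spawns a new BP_ImpCharacter at the saved checkpoint, or at the PlayerStart actor if none is set, and has player controller 0 possess it.
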(event EventBeginPlay)

(event EventTick
  (params (DeltaSeconds :type Float%20%28single-precision%29)))

(fn SetActiveCheckpoint
  (params (CheckpointTransform :type Transform))
  (Variables|Default|SetActiveCheckpointTransform CheckpointTransform)
  (Variables|Default|SetHasCheckpoint true))

(fn RespawnPlayer
  (if (Variables|Default|GetHasCheckpoint)
    (Actor|DestroyActor (Pawn|GetControlledPawn (Game|GetPlayerController 0)))
    (bind _returnvalue (Game|SpawnActorfromClass "/Game/ImpCharacter/demon_imp_v4/BP_ImpCharacter.BP_ImpCharacter_C" (Variables|Default|GetActiveCheckpointTransform) "Undefined" "MultiplyWithRoot" 0 0))
    (Pawn|Possess (Game|GetPlayerController 0) _returnvalue)
    (else
      (bind _returnvalue_2 (Actor|GetActorOfClass "/Script/Engine.PlayerStart"))
      (Actor|DestroyActor (Pawn|GetControlledPawn (Game|GetPlayerController 0)))
      (bind _returnvalue_3 (Game|SpawnActorfromClass "/Game/ImpCharacter/demon_imp_v4/BP_ImpCharacter.BP_ImpCharacter_C" (Transformation|GetActorTransform _returnvalue_2) "Undefined" "MultiplyWithRoot" 0 0))
      (Pawn|Possess (Game|GetPlayerController 0) _returnvalue_3))))