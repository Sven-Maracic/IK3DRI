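; Material swap component that overrides every material slot on TargetMesh with one material and can put cached ones back.
; ApplyMaterialToAllSlots first calls CacheOriginalMaterials, which fills OriginalMaterials only once, guarded by HasCachedMaterials.
; RestoreOriginalMaterials writes that array back by index.
; As written, caching skips slot 0 while restore starts there, so materials shift one slot and the restore loop overruns the array.
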(event EventBeginPlay)

(event EventTick
  (params (DeltaSeconds :type Float%20%28single-precision%29)))

(fn CacheOriginalMaterials
  (bind _targetmesh (Variables|Default|GetTargetMesh))
  (Utilities|IsValid _targetmesh
    (:Is%20Valid
      (if (not (Variables|Default|GetbHasCachedMaterials))
        (Utilities|Array|Clear (Variables|Default|GetOriginalMaterials))
        (for _index (range 1 (- (Rendering|Material|GetNumMaterials (Variables|Default|GetTargetMesh)) 1))
          (Utilities|Array|Add (Variables|Default|GetOriginalMaterials) (Rendering|Material|GetMaterial _targetmesh _index)))
        (Variables|Default|SetbHasCachedMaterials true)))))

(fn ApplyMaterialtoAllSlots
  (params (NewMaterial :type Material%20Interface%20Object%20Reference))
  (bind _targetmesh (Variables|Default|GetTargetMesh))
  (Utilities|IsValid _targetmesh
    (:Is%20Valid
      (CallFunction|CacheOriginalMaterials)
      (for _index (range 0 (- (Rendering|Material|GetNumMaterials _targetmesh) 1))
        (Rendering|Material|SetMaterial (Variables|Default|GetTargetMesh) _index NewMaterial)))))

(fn RestoreOriginalMaterials
  (bind _originalmaterials (Variables|Default|GetOriginalMaterials))
  (bind _returnvalue (Utilities|Array|Length _originalmaterials))
  (Utilities|IsValid (Variables|Default|GetTargetMesh)
    (:Is%20Valid
      (if (> _returnvalue 0)
        (for _index (range 0 (- _returnvalue -1))
          (Rendering|Material|SetMaterial (Variables|Default|GetTargetMesh) _index (Utilities|Array|Get(acopy) (Variables|Default|GetOriginalMaterials) _index)))))))