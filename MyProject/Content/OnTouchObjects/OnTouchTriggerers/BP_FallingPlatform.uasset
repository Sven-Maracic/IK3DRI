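; BP_FallingPlatform is a touch-triggered platform that drops away after a BP_ImpCharacter steps into its overlap.
; On begin overlap it waits a configurable delay, enables physics simulation on its Cube and sets a lifespan so the actor destroys itself.
; On end overlap it calls OnTouch on TouchEffectBase, passing the character and itself, so that effect fires as the character leaves rather than arrives.
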(event Collision|EventActorEndOverlap
  (params (OtherActor :type Actor%20Object%20Reference))
  (bind _asbp_imp_character (Utilities|Casting|CastToBP_ImpCharacter OtherActor))
  (Default|OnTouch (Variables|Default|GetTouchEffectBase) _asbp_imp_character self))

(event Collision|EventActorBeginOverlap
  (params (OtherActor :type Actor%20Object%20Reference))
  (Utilities|Casting|CastToBP_ImpCharacter OtherActor)
  (Utilities|FlowControl|Delay (Variables|Default|GetDelayDuration))
  (Physics|SetSimulatePhysics (Variables|Default|GetCube self) true)
  (Actor|SetLifeSpan (Variables|Default|GetIn%20Lifespan)))

(fn ConstructionScript
  (|CallParentFunction))